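; BP_PurgeRitual is a win-condition actor that ends the game in victory when the player enters its CompletionZone after the Captain has died.
; On overlap by the player character, it checks the referenced Captain's AshenAttributeComponent and requires that it reports not alive.
; It then sets RitualCompleted to prevent repeat triggers, shows the WBP_Victory widget and pauses the game.
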(event `self.CompletionZone.OnComponentBeginOverlap`
  (params (OverlappedComponent :type "PrimitiveComponent Object Reference") (OtherActor :type "Actor Object Reference") (OtherComp :type "PrimitiveComponent Object Reference") (OtherBodyIndex :type Integer) (bFromSweep :type Boolean) (SweepResult :type "HitResult Structure (by ref)"))
  (bind _captain (`self.Captain`))
  (cast `/Game/Characters/BP_AshenPlayerCharacter` OtherActor)
  (if (not (`self.bRitualCompleted`))
    (`/Engine/EditorBlueprintResources/StandardMacros.IsValid` _captain
      (:`Is Valid`
        (bind _asashen_attribute_component (cast `AshenAttributeComponent` (`self.GetComponentByClass` _captain "/Script/AshenKeep.AshenAttributeComponent")))
        (if (not (`AshenAttributeComponent.IsAlive` _asashen_attribute_component))
          (set `self.bRitualCompleted` true)
          (bind _returnvalue (`|CreateWidget` "/Game/WBP_Victory.WBP_Victory_C" (`GameplayStatics.GetPlayerController` 0)))
          (`UserWidget.AddToViewport` _returnvalue 0)
          (`GameplayStatics.SetGamePaused` true))))))

(fn `UserConstructionScript`)